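; Player character base with standard movement, yaw, jump and a prototype web-swing ability.
; Pressing CreateWeb grows the WebScan volume in a loop, then resets it; overlapping a WebPoint actor stores its location and starts swinging.
; While swinging, Tick sweeps the actor by its rotated offset from that point, but the zero axis and current-location base prevent a true orbit.
; Releasing CreateWeb ends the swing.
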(event EventBeginPlay)

(event Collision|EventActorBeginOverlap
  (params (OtherActor :type Actor%20Object%20Reference))
  ;[1 1 1] Scanning for web points
  (bind _asweb_point (Utilities|Casting|CastToWebPoint OtherActor))
  (Variables|Default|SetNotLatched false)
  (Variables|Default|SetSwingPosition (Transformation|GetActorLocation _asweb_point))
  (Development|PrintString "Found Point")
  (Variables|Default|SetSwinging true))

(event EventTick
  (params (DeltaSeconds :type Float%20%28single-precision%29))
  (bind _capsulecomponent (Variables|Collision|GetCapsuleComponent))
  (bind _returnvalue (Transformation|GetWorldLocation _capsulecomponent))
  (if (Variables|Default|GetSwinging)
    (Transformation|SetActorLocation (+ (Math|Vector|RotateVectorAroundAxis (- _returnvalue (Variables|Default|GetSwingPosition)) DeltaSeconds "0, 0, 0") _returnvalue) true false)))

(event Input|ActionEvents|InputActionJump
  (params (Key :type Key%20Structure))
  ;[1 1 1] Core Movement
  (:Pressed
    (Character|Jump)))

(event Input|ActionEvents|InputActionCreateWeb
  (params (Key :type Key%20Structure))
  ;[1 1 1] Core Movement
  (:Pressed
    (Variables|Default|SetNotLatched true)
    (CallFunction|ScanforPoints))
  (:Released
    (Variables|Default|SetNotLatched true)
    (Variables|Default|SetSwingPosition "0, 0, 0")
    (Variables|Default|SetSwinging false)))

(event Input|AxisEvents|InputAxisForward
  (params (AxisValue :type Float%20%28single-precision%29))
  ;[1 1 1] Core Movement
  (Pawn|Input|AddMovementInput (Math|Vector|GetForwardVector (Pawn|GetControlRotation :!class /Script/Engine.Pawn)) AxisValue false))

(event Input|AxisEvents|InputAxisRight
  (params (AxisValue :type Float%20%28single-precision%29))
  ;[1 1 1] Core Movement
  (Pawn|Input|AddMovementInput (Math|Vector|GetRightVector (Variables|Collision|GetCapsuleComponent)) AxisValue false))

(event Input|AxisEvents|InputAxisRotationX
  (params (AxisValue :type Float%20%28single-precision%29))
  ;[1 1 1] Core Movement
  (Pawn|Input|AddControllerYawInput AxisValue))

(fn ConstructionScript)

(fn ScanforPoints
  (bind _webscan (Variables|Default|GetWebScan))
  (while (and (Variables|Default|GetNotLatched) (< (Variables|Default|GetCurrentScanSize) (Variables|Default|GetmaxScanSize)))
    (Transformation|SetWorldScale3D _webscan (+ (Transformation|GetWorldScale _webscan) (Math|Vector|MakeVector 1.0 1.0 1.0)))
    (Variables|Default|SetCurrentScanSize (+ (Variables|Default|GetCurrentScanSize) 1.0)))
  (Transformation|SetWorldScale3D (Variables|Default|GetWebScan) "1.000000,1.000000,1.000000")
  (Variables|Default|SetCurrentScanSize 0.0)
  (Development|PrintString "Scanned"))